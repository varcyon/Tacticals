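; Grid visual actor that draws cells as instances of one InstancedStaticMesh, with mesh, material, base color and collision set at initialization.
; A parallel InstanceIndexes array maps grid indices to instances, so cells can be replaced, removed or cleared.
; Adding a cell converts its states, with Selected taking priority over Hovered, into per-instance custom data for RGB color and a filled flag.
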(event `self.ReceiveBeginPlay`
  (`self.SetActorTickEnabled` false))

(fn `AddInstance`
  (params (Transform :type "Transform Structure (by ref)") (Index :type "IntPoint Structure (by ref)") (States :type "Array of /Game/Core/Grid/Ultilities/E_TileState Enum"))
  (locals (i :type Integer :default 0))
  (`self.RemoveIntance` Index)
  (`InstancedStaticMeshComponent.AddInstance` (`self.InstancedStaticMesh`) Transform true)
  (bind _returnvalue (`KismetArrayLibrary.Array_Add` (`self.InstanceIndexes`) Index))
  (set `local.i` _returnvalue)
  (bind (_color _isfilled) (`self.GetColorFromStates` (`local.States`)))
  (bind (_r _g _b) (`KismetMathLibrary.BreakColor` _color))
  (`InstancedStaticMeshComponent.SetCustomDataValue` (`self.InstancedStaticMesh`) (`local.i`) 0 _r false)
  (`InstancedStaticMeshComponent.SetCustomDataValue` (`self.InstancedStaticMesh`) (`local.i`) 1 _g false)
  (`InstancedStaticMeshComponent.SetCustomDataValue` (`self.InstancedStaticMesh`) (`local.i`) 2 _b false)
  (`InstancedStaticMeshComponent.SetCustomDataValue` (`self.InstancedStaticMesh`) (`local.i`) 3 _isfilled false))

(fn `ClearInstances`
  (`InstancedStaticMeshComponent.ClearInstances` (`self.InstancedStaticMesh`))
  (`KismetArrayLibrary.Array_Clear` (`self.InstanceIndexes`)))

(fn `GetColorFromStates`
  (params (States :type "Array of /Game/Core/Grid/Ultilities/E_TileState Enum"))
  (returns (Color :type "LinearColor Structure") (IsFilled :type "Float (double-precision)"))
  (if (== (`KismetArrayLibrary.Array_Length` States) 0)
    (return (struct) 0.0)
    (else
      (for _array_element (`|MakeArray` "NewEnumerator2" "NewEnumerator1" :!type "/Game/Core/Grid/Ultilities/E_TileState Enum")
        (if (`KismetArrayLibrary.Array_Contains` (`local.States`) _array_element)
          (return (select `/Game/Core/Grid/Ultilities/E_TileState` _array_element :`NewEnumerator1` (struct :`R` 0.765625 :`G` 0.50923 :`A` 1.0) :`NewEnumerator2` (struct :`R` 0.91963 :`G` 0.103493 :`B` 1.0 :`A` 1.0) :!type "LinearColor Structure") 1.0)))
      (return (struct) 0.0))))

(fn `InitialGridMeshInst`
  (params (Mesh :type "StaticMesh Object Reference") (Material :type "MaterialInterface Object Reference") (Color :type "LinearColor Structure") (Collision :type "ECollisionEnabled Enum" :default "NoCollision"))
  (bind _instancedstaticmesh (`self.InstancedStaticMesh`))
  (`StaticMeshComponent.SetStaticMesh` _instancedstaticmesh Mesh)
  (`PrimitiveComponent.SetMaterial` _instancedstaticmesh 0 Material)
  (`MeshComponent.SetVectorParameterValueOnMaterials` _instancedstaticmesh "Color" (`KismetMathLibrary.Conv_LinearColorToVector` Color))
  (`PrimitiveComponent.SetCollisionEnabled` _instancedstaticmesh Collision))

(fn `RemoveIntance`
  (params (Index :type "IntPoint Structure (by ref)"))
  (bind _instanceindexes (`self.InstanceIndexes`))
  (if (`KismetArrayLibrary.Array_Contains` _instanceindexes Index)
    (`InstancedStaticMeshComponent.RemoveInstance` (`self.InstancedStaticMesh`) (`KismetArrayLibrary.Array_Find` _instanceindexes Index))
    (`KismetArrayLibrary.Array_RemoveItem` _instanceindexes Index)))

(fn `UserConstructionScript`)