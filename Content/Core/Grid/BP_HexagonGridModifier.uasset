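; Editor-placed grid modifier actor that marks a tile type (None, Normal, Obstacle, Double, Tripple or Flying) and is hidden in game.
; The construction script sets the mesh and flat material from the selected Shape's data, then tints it by Type through filled-material parameters.
; It sets the mesh to overlap on a custom trace channel, and has no active runtime logic.
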(fn `UserConstructionScript`
  (bind _staticmesh (`self.StaticMesh`))
  (bind (_out_row_meshsize _out_row_mesh _out_row_mestmaterial _out_row_flatmesh _out_row_flatmaterial) (break `/Game/Core/Grid/GridShapes/S_GridShape` (`/Game/Core/Grid/GridShapes/BFL_Gridshape.GetShapeData` (`self.Shape`))))
  (`StaticMeshComponent.SetStaticMesh` _staticmesh _out_row_mesh)
  (`PrimitiveComponent.SetMaterial` _staticmesh 0 _out_row_flatmaterial)
  (`MeshComponent.SetVectorParameterValueOnMaterials` _staticmesh "Color" (`KismetMathLibrary.Conv_LinearColorToVector` (select `/Game/Core/Grid/Ultilities/E_TileType` (`self.Type`) :`NewEnumerator1` (struct :`R` 1.0 :`G` 1.0 :`B` 1.0 :`A` 1.0) :`NewEnumerator2` (struct :`R` 1.0 :`G` 0.000133 :`B` 0.002519 :`A` 1.0) :`NewEnumerator3` (struct :`R` 0.363811 :`G` 0.341942 :`B` 1.0 :`A` 1.0) :`NewEnumerator4` (struct :`R` 1.0 :`G` 0.269987 :`B` 0.16416 :`A` 1.0) :`NewEnumerator5` (struct :`R` 0.109364 :`G` 1.0 :`B` 0.934522 :`A` 1.0) :!type "LinearColor Structure")))
  (`MeshComponent.SetScalarParameterValueOnMaterials` _staticmesh "IsFilled" 1.0)
  (`PrimitiveComponent.SetCollisionResponseToChannel` _staticmesh "ECC_GameTraceChannel1" "ECR_Overlap")
  (`self.SetActorHiddenInGame` true))