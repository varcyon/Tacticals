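; BP_Grid builds a square, triangle or hexagon tile grid as instanced static meshes around a center location.
; SpawnGrid clears old instances, applies the shape's mesh, snaps the center and bottom-left corner, then derives each tile's transform from its index.
; With UseEnvironment, sphere traces snap tile heights to the ground, read BP_GridModifier types and omit unwalkable tiles.
; The construction script's SpawnGrid call is disconnected.
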(fn `CalculatCenterAndBottomLeft`
  (returns (Center :type "Vector Structure") (BottomLeft :type "Vector Structure"))
  (locals (c :type "Vector Structure" :default (0.0 0.0 0.0)))
  (bind (_gridtile_count_x _gridtile_count_y) (`KismetMathLibrary.BreakVector2D` (`self.GridTile Count`)))
  (switch `/Game/Core/Grid/GridShapes/E_GridShapes` (`self.GridShape`)
    (:`NewEnumerator1`
      (set `local.c` (`/Game/Core/Utilities/BFL_Utilities.SnapVectorToVecter` (`self.GridCenter Location`) (`self.GridTile Size`)))
      (return (`local.c`) (- (`local.c`) (* (/ (- (`self.GridTile Count`) (`KismetMathLibrary.MakeVector2D` (`KismetMathLibrary.Conv_IntToDouble` (select `bool` (`self.IsFloatEven` _gridtile_count_x) :`false` 1)) (`KismetMathLibrary.Conv_IntToDouble` (select `bool` (`self.IsFloatEven` _gridtile_count_y) :`false` 1)))) 2.0) (`self.GridTile Size`)))))
    (:`NewEnumerator2`
      (set `local.c` (`/Game/Core/Utilities/BFL_Utilities.SnapVectorToVecter` (`self.GridCenter Location`) (* (`self.GridTile Size`) (2.0 1.0 1.0))))
      (return (`local.c`) (- (`local.c`) (`/Game/Core/Utilities/BFL_Utilities.SnapVectorToVecter` (* (/ (- (`self.GridTile Count`) (1.0 1.0)) (2.0 4.0)) (`self.GridTile Size`)) (* (`self.GridTile Size`) (2.0 1.0 1.0))))))
    (:`NewEnumerator3`
      (set `local.c` (`/Game/Core/Utilities/BFL_Utilities.SnapVectorToVecter` (`self.GridCenter Location`) (* (`self.GridTile Size`) (1.5 1.0 1.0))))
      (return (`local.c`) (- (`local.c`) (`/Game/Core/Utilities/BFL_Utilities.SnapVectorToVecter` (* (/ (`self.GridTile Count`) (3.0 2.0)) (`self.GridTile Size`)) (* (`self.GridTile Size`) (1.5 1.0 1.0))))))))

(fn `DestroyGrid`
  (`InstancedStaticMeshComponent.ClearInstances` (`self.InstancedStaticMesh`)))

(fn `GetCurrentShapeData`
  (returns (`Out Row` :type "/Game/Core/Grid/GridShapes/S_GridShape Structure"))
  (return (`/Game/Core/Grid/GridShapes/BFL_Gridshape.GetShapeData` (`self.GridShape`))))

(fn `GetTileLocationFromGridIndex`
  (params (GridIndex :type "Vector2D Structure"))
  (returns (TileLocation :type "Vector Structure"))
  (return (+ (`self.GridBottomLeftCornerLocation`) (* (`self.GridTile Size`) (* GridIndex (select `/Game/Core/Grid/GridShapes/E_GridShapes` (`self.GridShape`) :`NewEnumerator1` (1.0 1.0) :`NewEnumerator2` (1.0 0.5) :`NewEnumerator3` (0.75 0.5) :!type "Vector2D Structure"))))))

(fn `GetTileRotationFromGirdIndex`
  (params (GridIndex :type "Vector2D Structure"))
  (returns (TileRotation :type "Rotator Structure"))
  (bind (_gridindex_x _gridindex_y) (`KismetMathLibrary.BreakVector2D` (`local.GridIndex`)))
  (if (`|EnumEquality` (`self.GridShape`) "NewEnumerator2")
    (return (`KismetMathLibrary.MakeRotator` 0.0 0.0 (`KismetMathLibrary.Conv_IntToDouble` (+ (select `bool` (`self.IsFloatEven` _gridindex_x) :`true` 180) (select `bool` (`self.IsFloatEven` _gridindex_y) :`true` 180)))))
    (else
      (return))))

(fn `IsFloatEven`
  (params (Float :type "Float (double-precision)"))
  (returns (IsEven :type Boolean))
  (return (== (mod Float 2.0) 0.0)))

(fn `IsIntEven`
  (params (Float :type Integer))
  (returns (IsEven :type Boolean))
  (return (== (mod Float 2) 0)))

(fn `IsTileTypeWalkable`
  (params (Type :type "/Game/Core/Grid/Ultilities/E_TileType Enum" :default "NewEnumerator0"))
  (returns (Walkable :type Boolean))
  (return (not (`KismetArrayLibrary.Array_Contains` (`|MakeArray` "NewEnumerator0" "NewEnumerator2" :!type "/Game/Core/Grid/Ultilities/E_TileType Enum") Type))))

(fn `SpawnGrid`
  (params (CenterLocation :type "Vector Structure") (TileSize :type "Vector Structure") (TileCount :type "Vector2D Structure") (Shape :type "/Game/Core/Grid/GridShapes/E_GridShapes Enum" :default "NewEnumerator0") (UseEnvironment :type Boolean :default true))
  (locals (X :type Integer) (Y :type Integer) (TileTransform :type "Transform Structure") (index :type "Vector2D Structure"))
  (bind _out_row_meshsize (break `/Game/Core/Grid/GridShapes/S_GridShape` (`self.GetCurrentShapeData`)))
  (bind (_out_row_meshsize_2 _out_row_mesh _out_row_mestmaterial _out_row_flatmesh _out_row_flatbordermaterial) (break `/Game/Core/Grid/GridShapes/S_GridShape` (`self.GetCurrentShapeData`)))
  (bind _instancedstaticmesh (`self.InstancedStaticMesh`))
  (bind (_gridtile_count_x _gridtile_count_y) (`KismetMathLibrary.BreakVector2D` (`self.GridTile Count`)))
  (bind (_tiletransform_location _tiletransform_rotation _tiletransform_scale) (`KismetMathLibrary.BreakTransform` (`local.TileTransform`)))
  (bind (_gridtile_count_x_2 _gridtile_count_y_2) (`KismetMathLibrary.BreakVector2D` (`self.GridTile Count`)))
  (bind _gridtile_count_x_3 (`KismetMathLibrary.BreakVector2D` (`self.GridTile Count`)))
  (set `self.GridCenter Location` CenterLocation)
  (set `self.GridTile Size` TileSize)
  (set `self.GridShape` Shape)
  (set `self.GridTile Count` (`KismetMathLibrary.MakeVector2D` (`KismetMathLibrary.Conv_IntToDouble` (`KismetMathLibrary.Round` TileCount_X)) (`KismetMathLibrary.Conv_IntToDouble` (`KismetMathLibrary.Round` TileCount_Y))))
  (`self.DestroyGrid`)
  (`StaticMeshComponent.SetStaticMesh` _instancedstaticmesh _out_row_flatmesh)
  (`PrimitiveComponent.SetMaterial` _instancedstaticmesh 0 _out_row_flatbordermaterial)
  (bind (_center _bottomleft) (`self.CalculatCenterAndBottomLeft`))
  (set `self.GridCenter Location` _center)
  (set `self.GridBottomLeftCornerLocation` _bottomleft)
  (for _index (range (`KismetMathLibrary.Round` _gridtile_count_x_3))
    (set `local.X` _index)
    (if (`|EnumEquality` (`self.GridShape`) "NewEnumerator3")
      (for _index_2 (range (`KismetMathLibrary.SelectInt` 0 1 (`self.IsIntEven` (`local.X`))) (* (`KismetMathLibrary.Round` _gridtile_count_y_2) 2))
        (set `local.Y` _index_2)
        (`|ExecutionSequence`
          (:`then_0`
            (set `local.index` (`KismetMathLibrary.MakeVector2D` (`KismetMathLibrary.Conv_IntToDouble` (`local.X`)) (`KismetMathLibrary.Conv_IntToDouble` (`local.Y`))) :!label _label)
            (bind _output_get (set `local.TileTransform` (`KismetMathLibrary.MakeTransform` (+ (`self.GetTileLocationFromGridIndex` (`local.index`)) (0.0 0.0 2.0)) (`self.GetTileRotationFromGirdIndex` (`local.index`)) (/ (`self.GridTile Size`) _out_row_meshsize))))
            (set `local.TileTransform` _output_get)
            (if (`local.UseEnvironment`)
              (bind (_outlocation _tiletype) (`self.TraceForGround` _tiletransform_location))
              (bind _walkable (`self.IsTileTypeWalkable` _tiletype))
              (if _walkable
                (bind _output_get_2 (set `local.TileTransform` (`KismetMathLibrary.MakeTransform` (`KismetMathLibrary.MakeVector` (.x _outlocation) (.y _outlocation) (+ (.z _outlocation) 0.1)) _tiletransform_rotation _tiletransform_scale)))
                (`InstancedStaticMeshComponent.AddInstance` (`self.InstancedStaticMesh`) _output_get_2 true))
              (else
                (`InstancedStaticMeshComponent.AddInstance` (`self.InstancedStaticMesh`) (`local.TileTransform`) true))))
          (:`then_1`
            (`/Engine/EditorBlueprintResources/StandardMacros.IncrementInt` _index_2))))
      (else
        (for _index_3 (range (`KismetMathLibrary.Round` _gridtile_count_y))
          (set `local.Y` _index_3)
          (goto _label))))))

(fn `TraceForGround`
  (params (Location :type "Vector Structure"))
  (returns (OutLocation :type "Vector Structure") (TileType :type "/Game/Core/Grid/Ultilities/E_TileType Enum"))
  (locals (RetType :type "/Game/Core/Grid/Ultilities/E_TileType Enum" :default "NewEnumerator0") (RetZ :type "Float (double-precision)" :default 0.0))
  (bind _gridtile_size_x (`KismetMathLibrary.BreakVector` (`self.GridTile Size`)))
  (bind (_location_x _location_y) (`KismetMathLibrary.BreakVector` (`local.Location`)))
  (bind _location (`local.Location`))
  (bind (_gridtile_size_x_2 _gridtile_size_y _gridtile_size_z) (`KismetMathLibrary.BreakVector` (`self.GridTile Size`)))
  (set `self.Radius` (/ _gridtile_size_x (`KismetMathLibrary.SelectFloat` 5.0 3.0 (`|EnumEquality` (`self.GridShape`) "NewEnumerator2"))))
  (bind _outhits (`KismetSystemLibrary.SphereTraceMulti` (+ _location (0.0 0.0 1000.0)) (- _location (0.0 0.0 1000.0)) (`self.Radius`) "TraceTypeQuery3" true))
  (if (> (`KismetArrayLibrary.Array_Length` _outhits) 0)
    (set `local.RetType` "NewEnumerator1")
    (for _array_element _outhits
      (bind (_bblockinghit _binitialoverlap _time _distance _location_2 _impactpoint _normal _impactnormal _physmat _hitactor) (`GameplayStatics.BreakHitResult` _array_element))
      (bind _asbp_grid_modifier (cast `/Game/Core/Grid/BP_GridModifier` _hitactor)
        (:`then`
          (set `local.RetType` (`/Game/Core/Grid/BP_GridModifier.Type` _asbp_grid_modifier)))
        (:`CastFailed`
          (set `local.RetZ` (`KismetMathLibrary.GridSnap_Float` (- (.z _location_2) (`self.Radius`)) _gridtile_size_z)))))
    (return (`KismetMathLibrary.MakeVector` _location_x _location_y (`local.RetZ`)) (`local.RetType`))
    (else
      (return (`local.Location`) "NewEnumerator0"))))

(fn `UserConstructionScript`)