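; Combat system component on BP_Grid that tracks units in combat and keeps their grid placement in sync.
; Adding, removing or re-indexing a unit updates tile occupancy and the unit's Index, then moves the actor to its tile, with -9999 as the off-grid sentinel.
; Grid-generated and tile-updated events re-snap affected units, or remove and destroy those on unwalkable tiles.
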(event `self.ReceiveBeginPlay`
  (bind _asbp_grid (cast `/Game/Core/Grid/BP_Grid` (`self.GetOwner`)))
  (bind _output_get (set `self.Grid` _asbp_grid))
  (add `/Game/Core/Grid/BP_Grid.OnGridGenerated` _output_get (`|CreateDelegate` :!event `OnGridGenerated`))
  (add `/Game/Core/Grid/BP_Grid.OnTileDataUpdated` _output_get (`|CreateDelegate` :!event `OnTileDataUpdated`)))

(fn `AddUnitInCombat`
  (params (Unit :type "/Game/Core/Blueprints/Units/BP_Unit Object Reference") (Index :type "IntPoint Structure"))
  (`KismetArrayLibrary.Array_Add` (`self.UnitsInCombat`) Unit)
  (`self.SetUnitIndexOnGrid` Unit Index))

(fn `OnGridGenerated`
  (locals (CopyOfUnitsInCombat :type "Array of /Game/Core/Blueprints/Units/BP_Unit Object Reference"))
  (bind _output_get (set `local.CopyOfUnitsInCombat` (`self.UnitsInCombat`)))
  (for _array_element _output_get
    (bind _index (`/Game/Core/Blueprints/Units/BP_Unit.Index` _array_element))
    (if (`/Game/Core/Grid/BP_Grid.IsTileWalkable` (`self.Grid`) _index)
      (`self.SetUnitIndexOnGrid` _array_element _index)
      (else
        (`self.RemoveUnitInCombat` _array_element)))))

(fn `OnTileDataUpdated`
  (params (Index :type "IntPoint Structure"))
  (locals (CopyOfUnitsInCombat :type "Array of /Game/Core/Blueprints/Units/BP_Unit Object Reference"))
  (bind _output_get (set `local.CopyOfUnitsInCombat` (`self.UnitsInCombat`)))
  (for _array_element _output_get
    (bind _index (`/Game/Core/Blueprints/Units/BP_Unit.Index` _array_element))
    (if (`KismetMathLibrary.Equal_IntPointIntPoint` (`local.Index`) _index)
      (if (`/Game/Core/Grid/BP_Grid.IsTileWalkable` (`self.Grid`) _index)
        (`self.SetUnitIndexOnGrid` _array_element _index)
        (break)
        (else
          (`self.RemoveUnitInCombat` _array_element)
          (break))))))

(fn `RemoveUnitInCombat`
  (params (Unit :type "/Game/Core/Blueprints/Units/BP_Unit Object Reference") (DestroyUnit :type Boolean :default true))
  (`KismetArrayLibrary.Array_RemoveItem` (`self.UnitsInCombat`) Unit)
  (`self.SetUnitIndexOnGrid` Unit (make `IntPoint` -9999 -9999))
  (if (`local.DestroyUnit`)
    (`Actor.K2_DestroyActor` (`local.Unit`))))

(fn `SetUnitIndexOnGrid`
  (params (Unit :type "/Game/Core/Blueprints/Units/BP_Unit Object Reference") (Index :type "IntPoint Structure"))
  (locals (PreviousTile :type "/Game/Core/Grid/Ultilities/S_TileData Structure"))
  (bind (_value _returnvalue) (`BlueprintMapLibrary.Map_Find` (`/Game/Core/Grid/BP_Grid.GridTiles` (`self.Grid`)) (`local.Index`)))
  (`|ExecutionSequence`
    (:`then_0`
      (if (!= (`/Game/Core/Blueprints/Units/BP_Unit.Index` (`local.Unit`)) (`local.Index`))
        (`|ExecutionSequence`
          (:`then_0`
            (bind _output_get (set `local.PreviousTile` (`BlueprintMapLibrary.Map_Find` (`/Game/Core/Grid/BP_Grid.GridTiles` (`self.Grid`)) (`/Game/Core/Blueprints/Units/BP_Unit.Index` (`local.Unit`)))))
            (if (== (`.Unit_16_A00C6E354EBFA740678A3EAD5137629A` (break `/Game/Core/Grid/Ultilities/S_TileData` _output_get)) (`local.Unit`))
              (bind _structout (setmembers `/Game/Core/Grid/Ultilities/S_TileData` :`StructRef` (`local.PreviousTile`) :`Unit` null))
              (`BlueprintMapLibrary.Map_Add` (`/Game/Core/Grid/BP_Grid.GridTiles` (`self.Grid`)) (`.Index_7_49CF76EB4FA50F75CF50CF846E7F08C7` (break `/Game/Core/Grid/Ultilities/S_TileData` _structout)) _structout)))
          (:`then_1`
            (set `/Game/Core/Blueprints/Units/BP_Unit.Index` (`local.Index`) (`local.Unit`))
            (if (!= (`local.Index`) (make `IntPoint` -9999 -9999))
              (bind _structout_2 (setmembers `/Game/Core/Grid/Ultilities/S_TileData` :`StructRef` (`BlueprintMapLibrary.Map_Find` (`/Game/Core/Grid/BP_Grid.GridTiles` (`self.Grid`)) (`local.Index`)) :`Unit` (`local.Unit`)))
              (`BlueprintMapLibrary.Map_Add` (`/Game/Core/Grid/BP_Grid.GridTiles` (`self.Grid`)) (`.Index_7_49CF76EB4FA50F75CF50CF846E7F08C7` (break `/Game/Core/Grid/Ultilities/S_TileData` _structout_2)) _structout_2))))))
    (:`then_1`
      (`Actor.K2_SetActorLocation` (`local.Unit`) (select `bool` _returnvalue :`false` (-9999.0 -9999.0 -9999.0) :`true` (.location (`.Transform_9_1589FFEC44B2BB77E95BC89D78F3FEC9` (break `/Game/Core/Grid/Ultilities/S_TileData` _value)))) false false))))