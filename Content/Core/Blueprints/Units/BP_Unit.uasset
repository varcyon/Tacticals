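; BP_Unit is a unit actor with type-driven visuals and hover and selection highlighting.
; The construction script looks up default data for the UnitType to set the skeletal mesh and animation Blueprint.
; Hover and selection setters update the ColorMultiply material parameter, tinting selected units red and stacking brightness boosts.
; BeginPlay runs an endless test loop that cycles six animation states every three seconds through an anim instance message.
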(event `self.ReceiveBeginPlay`
  (`KismetSystemLibrary.Delay` 3.0 :!label _label)
  (bind _output_get (set `self.TestAnimIndex` (cast `/Game/Assets/Units/E_UnitAnimationState` (mod (+ (`self.TestAnimIndex`) 1) 6))))
  (message `/Game/Assets/Units/BPI_UnitAnimation.SetUnitAnimationState` (`SkeletalMeshComponent.GetAnimInstance` (`self.SkeletalMesh`)) _output_get)
  (goto _label))

(fn `SetIsHovered`
  (params (IsHovered :type Boolean))
  (set `self.IsHovered` IsHovered)
  (`self.UpdateVisualHoveredOrSelected`))

(fn `SetIsSelected`
  (params (IsSelected :type Boolean))
  (set `self.IsSelected` IsSelected)
  (`self.UpdateVisualHoveredOrSelected`))

(fn `UpdateVisualHoveredOrSelected`
  (`MeshComponent.SetVectorParameterValueOnMaterials` (`self.SkeletalMesh`) "ColorMultiply" (`KismetMathLibrary.Conv_LinearColorToVector` (* (* (select `bool` (`self.IsSelected`) :`false` (struct :`R` 1.0 :`G` 1.0 :`B` 1.0 :`A` 1.0) :`true` (struct :`R` 1.0 :`B` 0.036124 :`A` 1.0) :!type "LinearColor Structure") (select `bool` (`self.IsHovered`) :`false` 1.0 :`true` 10.0)) (select `bool` (`self.IsSelected`) :`false` 1.0 :`true` 10.0)))))

(fn `UserConstructionScript`
  (bind _skeletalmesh (`self.SkeletalMesh`))
  (bind _unitdata (`/Game/Assets/Units/Utilities/BFL_Units.GetDefaultUnitDataFromUnitType` (`self.UnitType`)))
  (set `SkeletalMeshComponent.SkeletalMeshAsset` (break `/Game/Assets/Units/Utilities/S_UnitDataAssets` (`.Assests_5_BF9E96124F9A49B0A7EE4CBDA23AB601` (break `/Game/Assets/Units/Utilities/S_UnitData` _unitdata))) _skeletalmesh)
  (`SkeletalMeshComponent.SetAnimInstanceClass` _skeletalmesh (`.AnimBP_8_5D7A7A204BF102D2A0569FA8E06B9EC7` (break `/Game/Assets/Units/Utilities/S_UnitDataAssets` (`.Assests_5_BF9E96124F9A49B0A7EE4CBDA23AB601` (break `/Game/Assets/Units/Utilities/S_UnitData` _unitdata))))))