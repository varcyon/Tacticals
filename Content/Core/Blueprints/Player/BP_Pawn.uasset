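; BP_Pawn is a player pawn that acts as a movable camera with pan, zoom and stepped rotation.
; On BeginPlay it adds the default Enhanced Input mapping context and seeds desired location, rotation and spring arm length.
; Input events only edit these targets: movement relative to facing, clamped zoom, and 45-degree rotation steps.
; Tick interpolates the actor transform and arm length toward them for smooth motion.
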(event `self.ReceiveBeginPlay`
  (bind _returnvalue (subsystem `EnhancedInputLocalPlayerSubsystem`))
  (`/Engine/EditorBlueprintResources/StandardMacros.IsValid` _returnvalue
    (:`Is Valid`
      (`EnhancedInputSubsystemInterface.AddMappingContext` _returnvalue "/Game/Core/Input/IMC_Default.IMC_Default" 0 (struct))
      (set `self.DesiredLocation` (`self.K2_GetActorLocation`))
      (set `self.DesieredZoom` (`SpringArmComponent.TargetArmLength` (`self.SpringArm`)))
      (set `self.Desired_Rotation` (`self.K2_GetActorRotation`)))))

(event `EnhancedInput|/Game/Core/Input/Actions/IA_Zoom`
  (params (ActionValue :type "Float (double-precision)") (ElapsedSeconds :type "Float (double-precision)") (TriggeredSeconds :type "Float (double-precision)") (InputAction :type "InputAction Object Reference" :default "/Game/Core/Input/Actions/IA_Zoom.IA_Zoom"))
  (:`Triggered`
    (set `self.DesieredZoom` (`KismetMathLibrary.FClamp` (+ (`self.DesieredZoom`) (* (* ActionValue (`self.ZoonSpeed`)) -1.0)) 100.0 5000.0))))

(event `self.ReceiveTick`
  (params (DeltaSeconds :type "Float (single-precision)"))
  (bind _springarm (`self.SpringArm`))
  (set `SpringArmComponent.TargetArmLength` (`KismetMathLibrary.FInterpTo` (`SpringArmComponent.TargetArmLength` _springarm) (`self.DesieredZoom`) DeltaSeconds 2.0) _springarm)
  (`self.K2_SetActorLocation` (`KismetMathLibrary.VInterpTo` (`self.K2_GetActorLocation`) (`self.DesiredLocation`) DeltaSeconds 2.0))
  (`self.K2_SetActorRotation` (`KismetMathLibrary.RInterpTo` (`self.K2_GetActorRotation`) (`self.Desired_Rotation`) DeltaSeconds 2.0)))

(event `EnhancedInput|/Game/Core/Input/Actions/IA_MoveCamera`
  (params (ActionValue :type "Vector2D Structure") (ElapsedSeconds :type "Float (double-precision)") (TriggeredSeconds :type "Float (double-precision)") (InputAction :type "InputAction Object Reference" :default "/Game/Core/Input/Actions/IA_MoveCamera.IA_MoveCamera"))
  (:`Triggered`
    (set `self.DesiredLocation` (+ (`self.DesiredLocation`) (* (`self.GetActorForwardVector`) (* ActionValue_X 40.0)) (* (`self.GetActorRightVector`) (* ActionValue_Y 40.0))))))

(event `EnhancedInput|/Game/Core/Input/Actions/IA_RotateCameraRight`
  (params (ActionValue :type Boolean) (ElapsedSeconds :type "Float (double-precision)") (TriggeredSeconds :type "Float (double-precision)") (InputAction :type "InputAction Object Reference" :default "/Game/Core/Input/Actions/IA_RotateCameraRight.IA_RotateCameraRight"))
  (:`Started`
    (set `self.Desired_Rotation` (`KismetMathLibrary.ComposeRotators` (`self.Desired_Rotation`) (struct :`Yaw` -45.0)))))

(event `EnhancedInput|/Game/Core/Input/Actions/IA_RotateCameraLeft`
  (params (ActionValue :type Boolean) (ElapsedSeconds :type "Float (double-precision)") (TriggeredSeconds :type "Float (double-precision)") (InputAction :type "InputAction Object Reference" :default "/Game/Core/Input/Actions/IA_RotateCameraLeft.IA_RotateCameraLeft"))
  (:`Started`
    (set `self.Desired_Rotation` (`KismetMathLibrary.ComposeRotators` (`self.Desired_Rotation`) (struct :`Yaw` 45.0)))))

(fn `UserConstructionScript`)