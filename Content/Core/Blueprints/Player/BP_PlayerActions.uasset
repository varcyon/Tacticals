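; Player input actor that turns mouse hover and clicks on the BP_Grid into pluggable tile actions.
; Each tick it updates the tile under the cursor, moving a tile state to it and firing OnHoveredTileChanged.
; Left and right clicks execute their selected action on that tile, repeating on each new tile while held.
; SetSelectedActions replaces both action actors by destroying and spawning them, then broadcasts the change.
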(event `self.ReceiveBeginPlay`
  (bind _returnvalue (`GameplayStatics.GetActorOfClass` "/Game/Core/Grid/BP_Grid.BP_Grid_C"))
  (bind _output_get (set `self.Grid` _returnvalue))
  (set `self.BPC Combat System` (`/Game/Core/Grid/BP_Grid.BPC_CombatSystem` _output_get))
  (`self.EnableInput` (`GameplayStatics.GetPlayerController` 0)))

(event `self.ReceiveTick`
  (params (DeltaSeconds :type "Float (single-precision)"))
  (`self.UpdateTileUnderCursor`))

(event `EnhancedInput|/Game/Core/Input/Actions/IA_LeftMouseButton`
  (params (ActionValue :type Boolean) (ElapsedSeconds :type "Float (double-precision)") (TriggeredSeconds :type "Float (double-precision)") (InputAction :type "InputAction Object Reference" :default "/Game/Core/Input/Actions/IA_LeftMouseButton.IA_LeftMouseButton"))
  (:`Started`
    (`self.UpdateTileUnderCursor`)
    (set `self.IsLeftClickDown` true)
    (`self.SelectedAction_LeftClick` :!label _label
      (:`then`
        (`/Game/Core/Blueprints/Player/Actions/BP_Action.ExecuteAction` (`self.SelectedAction_LeftClick`) (`self.HoveredTile`)))
      (:`else`)))
  (:`Canceled`
    (set `self.IsLeftClickDown` false :!label _label_2))
  (:`Completed`
    (goto _label_2)))

(event `OnHoveredTileChanged`
  (`|ExecutionSequence`
    (:`then_0`
      (if (`self.IsLeftClickDown`)
        (goto _label)))
    (:`then_1`
      (if (`self.IsRightClickDown`)
        (`self.SelectedAction_RightClick` :!label _label_3
          (:`then`
            (`/Game/Core/Blueprints/Player/Actions/BP_Action.ExecuteAction` (`self.SelectedAction_RightClick`) (`self.HoveredTile`)))
          (:`else`))))))

(event `EnhancedInput|/Game/Core/Input/Actions/IA_RightMouseButton`
  (params (ActionValue :type Boolean) (ElapsedSeconds :type "Float (double-precision)") (TriggeredSeconds :type "Float (double-precision)") (InputAction :type "InputAction Object Reference" :default "/Game/Core/Input/Actions/IA_RightMouseButton.IA_RightMouseButton"))
  (:`Started`
    (`self.UpdateTileUnderCursor`)
    (set `self.IsRightClickDown` true)
    (goto _label_3))
  (:`Canceled`
    (set `self.IsRightClickDown` false :!label _label_4))
  (:`Completed`
    (goto _label_4)))

(fn `SetSelectedActions`
  (params (LeftACtion :type "/Game/Core/Blueprints/Player/Actions/BP_Action Class Reference") (RightAction :type "/Game/Core/Blueprints/Player/Actions/BP_Action Class Reference"))
  (`|ExecutionSequence`
    (:`then_0`
      (bind _selectedaction_leftclick (`self.SelectedAction_LeftClick`)
        (:`then`
          (`self.K2_DestroyActor` _selectedaction_leftclick)
          (set `self.SelectedAction_LeftClick` null))
        (:`else`
          _))
      (if (`KismetSystemLibrary.IsValidClass` (`local.LeftACtion`))
        (bind _returnvalue (`|SpawnActorFromClass` (`local.LeftACtion`) (`KismetMathLibrary.MakeTransform` (0.0 0.0 0.0)) "AlwaysSpawn" "MultiplyWithRoot" null self null))
        (set `self.SelectedAction_LeftClick` _returnvalue)))
    (:`then_1`
      (bind _selectedaction_rightclick (`self.SelectedAction_RightClick`)
        (:`then`
          (`self.K2_DestroyActor` _selectedaction_rightclick)
          (set `self.SelectedAction_RightClick` null))
        (:`else`
          _))
      (if (`KismetSystemLibrary.IsValidClass` (`local.RightAction`))
        (bind _returnvalue_2 (`|SpawnActorFromClass` (`local.RightAction`) (`KismetMathLibrary.MakeTransform` (0.0 0.0 0.0)) "AlwaysSpawn" "MultiplyWithRoot" null self null))
        (set `self.SelectedAction_RightClick` _returnvalue_2)))
    (:`then_2`
      (`self.OnSelectedActionChanged` (`self.SelectedAction_LeftClick`) (`self.SelectedAction_RightClick`)))))

(fn `UpdateTileUnderCursor`
  (bind _index (`/Game/Core/Grid/BP_Grid.GetTileIndexUnderCursor` (`self.Grid`) 0))
  (if (!= _index (`self.HoveredTile`))
    (`/Game/Core/Grid/BP_Grid.RemoveStateToTile` (`self.Grid`) (`self.HoveredTile`) "NewEnumerator1")
    (set `self.HoveredTile` _index)
    (`/Game/Core/Grid/BP_Grid.AddStateToTile` (`self.Grid`) (`self.HoveredTile`) "NewEnumerator1")
    (`self.OnHoveredTileChanged`)))

(fn `UserConstructionScript`)